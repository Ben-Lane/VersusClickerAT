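; BP_Cube is a cube game element that animates its scale when clicked to give the player visual feedback.
; The construction script sets the Cube component's relative scale from CubeSize.
; ClickedCube resets that scale and plays a timeline from the start, multiplying its Size track by CubeSize as world scale, then restores the relative scale when finished.
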(event `self.ReceiveBeginPlay`)

(event `ClickedCube`
  ;[1 0.4792 0.4792] Alter the size of the cube upon clicking to feedback to the player the movement
  (`SceneComponent.SetRelativeScale3D` (`self.Cube`) (`KismetMathLibrary.Conv_DoubleToVector` (`self.CubeSize`)))
  (bind (_direction _size) (`Timeline|Timeline` :!via `PlayFromStart`)
    (:`Update`
      (`SceneComponent.SetWorldScale3D` (`self.Cube`) (`KismetMathLibrary.Conv_DoubleToVector` (* _size (`self.CubeSize`)))))
    (:`Finished`
      (`SceneComponent.SetRelativeScale3D` (`self.Cube`) (`KismetMathLibrary.Conv_DoubleToVector` (`self.CubeSize`))))))

(fn `UserConstructionScript`
  ;[1 1 1] Set Cube up with its given scale
  (`SceneComponent.SetRelativeScale3D` (`self.Cube`) (`KismetMathLibrary.Conv_DoubleToVector` (`self.CubeSize`))))