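; Main player controller for a streamer raffle clicker game, adding the viewer input mapping and initialising GM_MainGameMode on BeginPlay.
; Keys start the raffle, restart the level, toggle perspective and cycle example players for testing, mostly gated by the game mode's current event.
; In streamer perspective, left clicks line-trace for Player-tagged cubes, then AddScore raises the GameInstance score using BPCScoreHandler upgrade values with a random crit bonus.
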(event `Key|R`
  (params (Key :type "Key Structure"))
  ;[1 1 1] Game Restart Key
  (:`Pressed`
    (bind _asgm_main_game_mode (cast `/Game/GM_MainGameMode` (`GameplayStatics.GetGameMode`)))
    (if (`|EnumEquality` (`/Game/GM_MainGameMode.CurrentEvent` _asgm_main_game_mode) "NewEnumerator3")
      (bind _asbp_streamer_data_gi (cast `/Game/GameData/BP_StreamerDataGI` (`GameplayStatics.GetGameInstance`)))
      (set `/Game/GameData/BP_StreamerDataGI.RaffleVisibility` "Hidden" _asbp_streamer_data_gi)
      (set `/Game/GameData/BP_StreamerDataGI.StreamerScore` 0 _asbp_streamer_data_gi)
      (`GameplayStatics.OpenLevelBySoftObjectPtr` "/Game/Scenes/TestingScene.TestingScene"))))

(event `self.ReceiveBeginPlay`
  (bind _returnvalue (pcsubsystem `EnhancedInputLocalPlayerSubsystem` self))
  ;[1 1 1 1 34] Sets up player inputs
  (`/Engine/EditorBlueprintResources/StandardMacros.IsValid` _returnvalue
    (:`Is Valid`
      (`EnhancedInputSubsystemInterface.AddMappingContext` _returnvalue "/Game/Input/MC_Viewer.MC_Viewer" 0 (struct))
      (bind _asgm_main_game_mode (cast `/Game/GM_MainGameMode` (`GameplayStatics.GetGameMode`)))
      (bind _output_get (set `self.GameMode` _asgm_main_game_mode))
      (`/Game/GM_MainGameMode.InitialiseGame` _output_get (`PlayerCameraManager.GetOwningPlayerController` (`self.PlayerCameraManager`))))))

(event `Key|Right`
  (params (Key :type "Key Structure"))
  (bind _gamemode (`self.GameMode`))
  (bind _gamemode_2 (`self.GameMode`))
  ;[1 0.8128 0 1 34] Control Player Cycling For Testing
  ;;[1 1 1] Cycle Player To The Right
  (:`Pressed`
    (bind _output_get (set `/Game/GM_MainGameMode.SelectedPlayer` (+ (`/Game/GM_MainGameMode.SelectedPlayer` _gamemode) 1) _gamemode_2))
    (if (>= _output_get (`KismetArrayLibrary.Array_Length` (`/Game/GM_MainGameMode.ExamplePlayers` _gamemode)))
      (set `/Game/GM_MainGameMode.SelectedPlayer` 0 _gamemode_2))
    (`/Game/GM_MainGameMode.UpdateCurrentPlayer` _gamemode_2)))

(event `Key|SpaceBar`
  (params (Key :type "Key Structure"))
  ;[1 1 1 1 58] Game Inputs
  (:`Pressed`
    (bind _asgm_main_game_mode (cast `/Game/GM_MainGameMode` (`GameplayStatics.GetGameMode`)))
    (if (and (`/Game/GM_MainGameMode.StreamerPerspective` _asgm_main_game_mode) (`|EnumEquality` (`/Game/GM_MainGameMode.CurrentEvent` _asgm_main_game_mode) "NewEnumerator0"))
      (`/Game/GM_MainGameMode.StartRaffle` _asgm_main_game_mode self))))

(event `Key|Left`
  (params (Key :type "Key Structure"))
  (bind _gamemode (`self.GameMode`))
  (bind _gamemode_2 (`self.GameMode`))
  ;[1 0.8128 0 1 34] Control Player Cycling For Testing
  ;;[1 1 1] Cycle Players To The Left
  (:`Pressed`
    (bind _output_get (set `/Game/GM_MainGameMode.SelectedPlayer` (- (`/Game/GM_MainGameMode.SelectedPlayer` _gamemode_2) 1) _gamemode))
    (if (< _output_get 0)
      (set `/Game/GM_MainGameMode.SelectedPlayer` (- (`KismetArrayLibrary.Array_Length` (`/Game/GM_MainGameMode.ExamplePlayers` _gamemode_2)) 1) _gamemode))
    (`/Game/GM_MainGameMode.UpdateCurrentPlayer` _gamemode)))

(event `Key|P`
  (params (Key :type "Key Structure"))
  ;[1 1 1 1 58] Game Inputs
  (:`Pressed`
    (bind _asgm_main_game_mode (cast `/Game/GM_MainGameMode` (`GameplayStatics.GetGameMode`)))
    (if true
      (`/Game/GM_MainGameMode.TogglePerspective` _asgm_main_game_mode))))

(event `Key|LeftMouseButton`
  (params (Key :type "Key Structure"))
  (bind _gamemode (`self.GameMode`))
  (bind (_worldlocation _worlddirection) (`self.DeprojectMousePositionToWorld` (`PlayerCameraManager.GetOwningPlayerController` (`self.PlayerCameraManager`))))
  ;[1 0.4063 0 1 26] Handles detection of clickable object, activating any required changes after doing so (shape change, score increment)
  (:`Pressed`
    (if (and (`/Game/GM_MainGameMode.StreamerPerspective` _gamemode) (`|EnumEquality` (`/Game/GM_MainGameMode.CurrentEvent` _gamemode) "NewEnumerator2"))
      (if (`/Game/GM_MainGameMode.StreamerParticipating` _gamemode)
        ;;[1 1 1] Handles Detection if in streamer perspective
        (bind _outhit (`KismetSystemLibrary.LineTraceSingle` (+ _worldlocation (* _worlddirection 10.0)) (+ _worldlocation (* _worlddirection 1000.0)) "TraceTypeQuery1"))
        (bind _asbp_cube (cast `/Game/GameElements/BP_Cube` (`.HitActor` (`GameplayStatics.BreakHitResult` _outhit))))
        (if (`self.ActorHasTag` _asbp_cube "Player")
          (`/Game/GameElements/BP_Cube.ClickedCube` _asbp_cube)
          (`self.AddScore`))))))

(fn `AddScore`
  (bind _bpc_scorehandler (`self.BPC_ScoreHandler`))
  (bind _bpc_scorehandler_2 (`self.BPC_ScoreHandler`))
  (bind _bpc_scorehandler_3 (`self.BPC_ScoreHandler`))
  (bind _upgradevalues (`/Game/BPC_ScoreHandler.UpgradeValues` _bpc_scorehandler_2))
  (bind _asbp_streamer_data_gi (cast `/Game/GameData/BP_StreamerDataGI` (`GameplayStatics.GetGameInstance`)))
  (set `/Game/GameData/BP_StreamerDataGI.StreamerScore` (+ (`/Game/GameData/BP_StreamerDataGI.StreamerScore` _asbp_streamer_data_gi) (`|GetArrayItem` (`/Game/BPC_ScoreHandler.UpgradeValues` _bpc_scorehandler) (`/Game/BPC_ScoreHandler.ClickValueBI` _bpc_scorehandler))) _asbp_streamer_data_gi)
  ;[1 1 1] Check Crit Chance
  (if (<= (`KismetMathLibrary.RandomFloatInRange` 0.0 100.0) (`|GetArrayItem` (`/Game/BPC_ScoreHandler.UpgradeValues` _bpc_scorehandler_3) (`/Game/BPC_ScoreHandler.CritChanceBI` _bpc_scorehandler_3)))
    (`/Game/UI/GeneralUI/WB_StreamerHUD.ShowCrit` (`/Game/GM_MainGameMode.StreamerHUD` (`self.GameMode`)) (`self.BPC_ScoreHandler`))
    ;[1 1 1] Add Score To player
    (bind _asbp_streamer_data_gi_2 (cast `/Game/GameData/BP_StreamerDataGI` (`GameplayStatics.GetGameInstance`)))
    (set `/Game/GameData/BP_StreamerDataGI.StreamerScore` (+ (`/Game/GameData/BP_StreamerDataGI.StreamerScore` _asbp_streamer_data_gi_2) (* (`|GetArrayItem` _upgradevalues (`/Game/BPC_ScoreHandler.CritValueBI` _bpc_scorehandler_2)) (`|GetArrayItem` _upgradevalues (`/Game/BPC_ScoreHandler.ClickValueBI` _bpc_scorehandler_2)))) _asbp_streamer_data_gi_2))
  (return))

(fn `UserConstructionScript`)