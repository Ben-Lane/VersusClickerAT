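; Score manager Blueprint that gives each player in GM_MainGameMode's ExamplePlayers array its own score calculation component.
; InitialisePlayers adds a BPC_ScoreHandler per entry, with the array index as ID, and writes it back into that player's struct as its ScoreCalculator.
; EnableCalculation starts every handler component, also calling StartCalculation on the game mode's CurrentScoreHandler on each loop pass.
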(event `InitialisePlayers`
  ;[1 1 1] Create score calculating player components
  (bind _asgm_main_game_mode (cast `/Game/GM_MainGameMode` (`GameplayStatics.GetGameMode`)))
  (for (_array_element _array_index) (`/Game/GM_MainGameMode.ExamplePlayers` _asgm_main_game_mode)
    (bind _returnvalue (`|AddComponentByClass` self "/Game/BPC_ScoreHandler.BPC_ScoreHandler_C" _array_index))
    (bind (_username _profilepicture _id _score _scoreaddition _participating) (break `/Game/GameData/STRUCT_Viewer` _array_element))
    (`KismetArrayLibrary.Array_Set` (`/Game/GM_MainGameMode.ExamplePlayers` _asgm_main_game_mode) _array_index (make `/Game/GameData/STRUCT_Viewer` _username _profilepicture _id _score _scoreaddition _participating _returnvalue))))

(fn `EnableCalculation`
  (for _array_element (`self.K2_GetComponentsByClass` self "/Game/BPC_ScoreHandler.BPC_ScoreHandler_C")
    (`/Game/BPC_ScoreHandler.StartCalculation` _array_element)
    (bind _asgm_main_game_mode (cast `/Game/GM_MainGameMode` (`GameplayStatics.GetGameMode`)))
    (`/Game/BPC_ScoreHandler.StartCalculation` (`/Game/GM_MainGameMode.CurrentScoreHandler` _asgm_main_game_mode))))

(fn `UserConstructionScript`)