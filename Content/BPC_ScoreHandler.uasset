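; Per-participant score component for a raffle game, adding lag, auto-click and crit points to the streamer (negative ID) or a player.
; BeginPlay seeds UpgradeValues from the score manager's curve tables after a short delay.
; StartCalculation starts looping lag and auto-click timers that score only while participating, restarting at new speeds when flagged.
; AddCritToPlayer adds crit points separately, checking participation only for players.
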(event `self.ReceiveBeginPlay`
  ;[1 1 1] Initialise UpgradeValues
  (`KismetSystemLibrary.Delay` 0.2)
  (bind _asgm_main_game_mode (cast `/Game/GM_MainGameMode` (`GameplayStatics.GetGameMode`)))
  (for (_array_element _array_index) (`/Game/BP_ScoreManager.UpgradeCurves` (`/Game/GM_MainGameMode.ScoreManager` _asgm_main_game_mode))
    (bind _returnvalue (`|GetDataTableRow` _array_element (`KismetStringLibrary.Conv_StringToName` "Upgrade0"))
      (:`then`
        (`KismetArrayLibrary.Array_Set` (`self.UpgradeValues`) _array_index (`.Value_3_E651CE44475AE76407647494F74AE900` (break `/Game/GameData/UpgradeCurves/STRUCT_UpgradeCurve` _returnvalue)))))))

(event `WipeLagTimer`
  (`KismetSystemLibrary.K2_ClearAndInvalidateTimerHandle` (stale `StartCalculation` _returnvalue)))

(event `WipeAutoTimer`
  (`KismetSystemLibrary.K2_ClearAndInvalidateTimerHandle` (stale `StartCalculation` _returnvalue_2)))

(event `StartCalculation`
  ;[1 1 1] Sets up the score increment function to happen on a timer (15 IS DEFAULT)
  ;;[1 0.2247 0.991] LAG SCORE
  (bind _returnvalue (`KismetSystemLibrary.K2_SetTimer` null "UpdateLagScore" (`KismetMathLibrary.Conv_IntToDouble` (`|GetArrayItem` (`self.UpgradeValues`) (`self.LagSpeedBI`))) true))
  ;;[1 0.2247 0.991] AUTO CLICK SCORE
  (bind _returnvalue_2 (`KismetSystemLibrary.K2_SetTimer` null "UpdateAutoClickScore" (`KismetMathLibrary.Conv_IntToDouble` (`|GetArrayItem` (`self.UpgradeValues`) (`self.AutoClickSpeedBI`))) true)))

(event `UpdateLagScore`
  ;[0.6911 1 0.2028 1 34] Add Score increment to player score, if the player is participating in the raffle
  (if (< (`self.ID`) 0)
    (bind _asgm_main_game_mode (cast `/Game/GM_MainGameMode` (`GameplayStatics.GetGameMode`)))
    (if (`/Game/GM_MainGameMode.StreamerParticipating` _asgm_main_game_mode)
      (bind _asbp_streamer_data_gi (cast `/Game/GameData/BP_StreamerDataGI` (`GameplayStatics.GetGameInstance`)))
      (set `/Game/GameData/BP_StreamerDataGI.StreamerScore` (+ (`/Game/GameData/BP_StreamerDataGI.StreamerScore` _asbp_streamer_data_gi) (* (`|GetArrayItem` (`self.UpgradeValues`) (`self.ClickValueBI`)) (`|GetArrayItem` (`self.UpgradeValues`) (`self.LagValueBI`)))) _asbp_streamer_data_gi)
      (`self.CheckLagTimerValidity` :!label _label))
    (else
      (bind _asgm_main_game_mode_2 (cast `/Game/GM_MainGameMode` (`GameplayStatics.GetGameMode`)))
      (bind _exampleplayers (`/Game/GM_MainGameMode.ExamplePlayers` _asgm_main_game_mode_2))
      (bind (_output_username _output_profilepicture _output_id _output_score _output_scoreaddition _output_participating _output_scorecalculator) (break `/Game/GameData/STRUCT_Viewer` (`|GetArrayItem` _exampleplayers (`self.ID`))))
      (if _output_participating
        (`KismetArrayLibrary.Array_Set` _exampleplayers _output_id (make `/Game/GameData/STRUCT_Viewer` _output_username _output_profilepicture _output_id (+ _output_score (* (`|GetArrayItem` (`self.UpgradeValues`) (`self.ClickValueBI`)) (`|GetArrayItem` (`self.UpgradeValues`) (`self.LagValueBI`)))) _output_scoreaddition _output_participating _output_scorecalculator))
        (goto _label)))))

(event `UpdateAutoClickScore`
  ;[0.6911 1 0.2028 1 34] Add Score increment to player score, if the player is participating in the raffle
  (if (< (`self.ID`) 0)
    (bind _asgm_main_game_mode (cast `/Game/GM_MainGameMode` (`GameplayStatics.GetGameMode`)))
    (if (`/Game/GM_MainGameMode.StreamerParticipating` _asgm_main_game_mode)
      (bind _asbp_streamer_data_gi (cast `/Game/GameData/BP_StreamerDataGI` (`GameplayStatics.GetGameInstance`)))
      (set `/Game/GameData/BP_StreamerDataGI.StreamerScore` (+ (`/Game/GameData/BP_StreamerDataGI.StreamerScore` _asbp_streamer_data_gi) (`|GetArrayItem` (`self.UpgradeValues`) (`self.AutoClickValueBI`))) _asbp_streamer_data_gi)
      (`self.CheckAutoTimerValidity` :!label _label_2))
    (else
      (bind _asgm_main_game_mode_2 (cast `/Game/GM_MainGameMode` (`GameplayStatics.GetGameMode`)))
      (bind _exampleplayers (`/Game/GM_MainGameMode.ExamplePlayers` _asgm_main_game_mode_2))
      (bind (_output_username _output_profilepicture _output_id _output_score _output_scoreaddition _output_participating _output_scorecalculator) (break `/Game/GameData/STRUCT_Viewer` (`|GetArrayItem` _exampleplayers (`self.ID`))))
      (if _output_participating
        (`KismetArrayLibrary.Array_Set` _exampleplayers _output_id (make `/Game/GameData/STRUCT_Viewer` _output_username _output_profilepicture _output_id (+ _output_score (`|GetArrayItem` (`self.UpgradeValues`) (`self.AutoClickValueBI`))) _output_scoreaddition _output_participating _output_scorecalculator))
        (goto _label_2)))))

(fn `AddCritToPlayer`
  (if (< (`self.ID`) 0)
    (bind _asbp_streamer_data_gi (cast `/Game/GameData/BP_StreamerDataGI` (`GameplayStatics.GetGameInstance`)))
    (set `/Game/GameData/BP_StreamerDataGI.StreamerScore` (+ (`/Game/GameData/BP_StreamerDataGI.StreamerScore` _asbp_streamer_data_gi) (`|GetArrayItem` (`self.UpgradeValues`) (`self.CritValueBI`))) _asbp_streamer_data_gi)
    (else
      (bind _asgm_main_game_mode (cast `/Game/GM_MainGameMode` (`GameplayStatics.GetGameMode`)))
      (bind _exampleplayers (`/Game/GM_MainGameMode.ExamplePlayers` _asgm_main_game_mode))
      (bind (_output_username _output_profilepicture _output_id _output_score _output_scoreaddition _output_participating) (break `/Game/GameData/STRUCT_Viewer` (`|GetArrayItem` _exampleplayers (`self.ID`))))
      (if _output_participating
        (`KismetArrayLibrary.Array_Set` _exampleplayers _output_id (make `/Game/GameData/STRUCT_Viewer` _output_username _output_profilepicture _output_id (+ _output_score (`|GetArrayItem` (`self.UpgradeValues`) (`self.CritValueBI`))) _output_scoreaddition _output_participating))))))

(fn `CheckAutoTimerValidity`
  (if (`self.AutoTimerNeedsUpdating`)
    (set `self.AutoTimerNeedsUpdating` false)
    (`self.WipeAutoTimer`)
    ;[1 0.2247 0.991] AUTO CLICK SCORE
    (`KismetSystemLibrary.K2_SetTimer` null "UpdateAutoClickScore" (`KismetMathLibrary.Conv_IntToDouble` (`|GetArrayItem` (`self.UpgradeValues`) (`self.AutoClickSpeedBI`))) true)))

(fn `CheckLagTimerValidity`
  (if (`self.LagTimerNeedsUpdating`)
    (set `self.LagTimerNeedsUpdating` false)
    (`self.WipeLagTimer`)
    ;[1 0.2247 0.991] LAG SCORE
    (`KismetSystemLibrary.K2_SetTimer` null "UpdateLagScore" (`KismetMathLibrary.Conv_IntToDouble` (`|GetArrayItem` (`self.UpgradeValues`) (`self.LagSpeedBI`))) true)))