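; Game mode for a streamer-and-viewer game prototype where example viewers enter a raffle, then compete on score with elimination.
; Builds both HUDs, player icons and a score manager, and toggles perspective, which pauses or resumes the raffle countdown.
; An event enum tracks the phase; raffle entrants gain access, starting scoring and elimination.
; During one phase, Tick re-ranks participants every frame (the half-second throttle is unwired), feeding the top four and elimination component.
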(event `GameEnd`
  (set `self.CurrentEvent` "NewEnumerator3")
  (`KismetSystemLibrary.PrintString` "Game ended"))

(event `self.ReceiveBeginPlay`
  (set `self.CurrentEvent` "NewEnumerator0")
  (set `self.JustChangedPlayer` false))

(event `TogglePerspective`
  (bind _viewerhud (`self.ViewerHUD`))
  (bind _bpc_rafflehandling (`self.BPC_RaffleHandling`))
  ;[1 1 1] Toggles between streamer and viewer view
  (`/Engine/EditorBlueprintResources/StandardMacros.FlipFlop`
    (:`A`
      (set `self.StreamerPerspective` true)
      (set `Widget.Visibility` "Hidden" _viewerhud)
      (`/Game/BPC_RaffleHandling.ContinueRaffleCountdown` _bpc_rafflehandling)
      (bind _asbp_main_player_controller (cast `/Game/BP_MainPlayerController` (`self.Controller`)))
      (set `self.CurrentScoreHandler` (`/Game/BP_MainPlayerController.BPC_ScoreHandler` _asbp_main_player_controller)))
    (:`B`
      (set `self.StreamerPerspective` false)
      (set `Widget.Visibility` "Visible" _viewerhud)
      (`/Game/BPC_RaffleHandling.StopRaffleCountdown` _bpc_rafflehandling))))

(event `self.ReceiveTick`
  (params (DeltaSeconds :type "Float (single-precision)"))
  ;[0.6454 0.1314 1] Update Leaderboard
  (if (`|EnumEquality` (`self.CurrentEvent`) "NewEnumerator2")
    (`self.UpdateLB`)
    (set `self.ElapsedTime` 0.0)))

(fn `Create Player Icons`
  ;[1 1 1 1 25] If the player icons have not been generated, it will create the visual to represent the current player selected, using player structures to obtain their player profile picture
  (for _array_element (`self.ExamplePlayers`)
    (`/Game/UI/GeneralUI/WB_PlayerIconDisplay.Add Images` (`/Game/UI/ViewerExclusive/WB_ViewerPerspective.PlayerIconsBox` (`self.ViewerHUD`)) (`self.Controller`) (`.ProfilePicture_5_6C02CA1F49D60221A1186BB5F748B16F` (break `/Game/GameData/STRUCT_Viewer` _array_element))))
  (`self.UpdateCurrentPlayer`))

(fn `EnterRaffle`
  (returns (NewEntry :type Boolean))
  (locals (PlayerAlreadyEntered :type Boolean))
  (bind (_output_username _output_profilepicture _output_id _output_score _output_scoreaddition _output_participating _output_scorecalculator) (break `/Game/GameData/STRUCT_Viewer` (`|GetArrayItem` (`self.ExamplePlayers`) (`self.SelectedPlayer`))))
  ;[1 1 1] Add To Raffle
  (if (`|EnumEquality` (`/Game/UI/ViewerExclusive/WB_Raffle.State` (`/Game/UI/GeneralUI/WB_StreamerHUD.WB_Raffle` (`self.StreamerHUD`))) "NewEnumerator0")
    (if _output_participating
      _
      (else
        (`KismetArrayLibrary.Array_Set` (`self.ExamplePlayers`) (`self.SelectedPlayer`) (make `/Game/GameData/STRUCT_Viewer` _output_username _output_profilepicture _output_id _output_score _output_scoreaddition true _output_scorecalculator))
        (`/Game/UI/ViewerExclusive/WB_Raffle.PlayerEntered` (`/Game/UI/GeneralUI/WB_StreamerHUD.WB_Raffle` (`self.StreamerHUD`)))
        (`/Game/UI/ViewerExclusive/WB_Raffle.PlayerEntered` (`/Game/UI/GeneralUI/WB_StreamerHUD.WB_Raffle` (`/Game/UI/ViewerExclusive/WB_ViewerHUD.WB_StreamerHUD` (`/Game/UI/ViewerExclusive/WB_ViewerPerspective.WB_ViewerHUD` (`self.ViewerHUD`)))))
        (return true))))
  (return false))

(fn `GiveViewersAccess`
  (locals (PlayersParticipating :type Integer))
  (bind _topplayers (`self.TopPlayers`))
  (for (_array_element _array_index) (`self.ExamplePlayers`)
    (if (`.Participating_16_2FB093A24519A01D14EE788F67F6B3C1` (break `/Game/GameData/STRUCT_Viewer` _array_element))
      (bind _aswb_icon (cast `/Game/UI/GeneralUI/WB_Icon` (`PanelWidget.GetChildAt` (`/Game/UI/GeneralUI/WB_PlayerIconDisplay.PictureLine` (`/Game/UI/ViewerExclusive/WB_ViewerPerspective.PlayerIconsBox` (`self.ViewerHUD`))) _array_index)))
      (bind _playingborder (`/Game/UI/GeneralUI/WB_Icon.PlayingBorder` _aswb_icon))
      (bind _background (`Border.Background` _playingborder))
      (`Border.SetBrush` _playingborder (make `SlateBrush` (break `SlateBrush` _background) (`.Tiling` (break `SlateBrush` _background)) (`.Mirroring` (break `SlateBrush` _background)) (`.ImageSize` (break `SlateBrush` _background)) (`.Margin` (break `SlateBrush` _background)) (make `SlateColor` (make `LinearColor` 0.0 1.0 0.0)) (`.OutlineSettings` (break `SlateBrush` _background)) (`.ResourceObject` (break `SlateBrush` _background))))
      ;[1 1 1] ADD TO LIST OF TOP 4 PLAYERS
      (if (< (`KismetArrayLibrary.Array_Length` _topplayers) 4)
        (`KismetArrayLibrary.Array_Add` _topplayers (`.ID_8_BA49C3F345E774A3080E77B342852339` (break `/Game/GameData/STRUCT_Viewer` _array_element))))))
  (`/Game/BP_ScoreManager.EnableCalculation` (`self.ScoreManager`))
  (`/Game/BPC_Elimination.StartEliminationProcess` (`self.BPC_Elimination`)))

(fn `InitialiseGame`
  (params (Player :type "PlayerController Object Reference"))
  ;[1 0.2244 0 1 26] This creates all widgets that will be default in the project, as well as any setup needed.
  (bind _output_get (set `self.Controller` Player))
  (bind _returnvalue (`|CreateWidget` "/Game/UI/GeneralUI/WB_StreamerHUD.WB_StreamerHUD_C" _output_get self))
  (bind _output_get_2 (set `self.StreamerHUD` _returnvalue))
  (`UserWidget.AddToPlayerScreen` _output_get_2 0)
  (bind _returnvalue_2 (`|CreateWidget` "/Game/UI/ViewerExclusive/WB_ViewerPerspective.WB_ViewerPerspective_C" Player self))
  (bind _output_get_3 (set `self.ViewerHUD` _returnvalue_2))
  (`UserWidget.AddToPlayerScreen` _output_get_3 0)
  (set `PlayerController.bShowMouseCursor` true Player)
  (set `self.StreamerPerspective` false)
  (`self.Create Player Icons`)
  (bind _returnvalue_3 (`|SpawnActorFromClass` "/Game/BP_ScoreManager.BP_ScoreManager_C" (`KismetMathLibrary.MakeTransform` (0.0 0.0 0.0)) "Undefined" "MultiplyWithRoot" null null))
  (bind _output_get_4 (set `self.ScoreManager` _returnvalue_3))
  (`/Game/BP_ScoreManager.InitialisePlayers` _output_get_4)
  (bind _asbp_main_player_controller (cast `/Game/BP_MainPlayerController` (`self.Controller`)))
  (set `self.CurrentScoreHandler` (`/Game/BP_MainPlayerController.BPC_ScoreHandler` _asbp_main_player_controller))
  (set `self.JustChangedPlayer` true))

(fn `InputPlayerLB`
  (params (StartingElement :type Integer))
  (locals (SavedValue :type Integer))
  (for _index (range (- (`KismetArrayLibrary.Array_Length` (`self.TopPlayers`)) 1) (+ StartingElement 1))
    (if (> _index StartingElement)
      (`KismetArrayLibrary.Array_Set` (`self.TopPlayers`) _index (`|GetArrayItem` (`self.TopPlayers`) (- _index 1))))))

(fn `PlayerInLB`
  (params (ID :type Integer))
  (returns (AlreadyInLB :type Boolean))
  (locals (AlreadyExists :type Boolean))
  (set `local.AlreadyExists` false)
  (for _array_element (`self.TopPlayers`)
    (bind _returnvalue (== _array_element ID))
    (if _returnvalue
      (set `local.AlreadyExists` _returnvalue)
      (break)))
  (return (`local.AlreadyExists`)))

(fn `StartRaffle`
  (params (Host :type "/Game/BP_MainPlayerController Object Reference"))
  (locals (NewLocalVar :type "/Game/UI/ViewerExclusive/WB_Raffle Object Reference"))
  ;[1 1 1 1 26] If a raffle doesnt already exist, one will be made, changing the state of this blueprint to say so
  (if (`|EnumInequality` (`self.CurrentEvent`) "NewEnumerator1")
    (set `self.CurrentEvent` "NewEnumerator1")
    (`KismetSystemLibrary.PrintString` "Raffle Started")
    (bind _asbp_streamer_data_gi (cast `/Game/GameData/BP_StreamerDataGI` (`GameplayStatics.GetGameInstance`)))
    (set `/Game/GameData/BP_StreamerDataGI.RaffleVisibility` "Visible" _asbp_streamer_data_gi)
    (if (`self.StreamerPerspective`)
      (`/Game/BPC_RaffleHandling.ContinueRaffleCountdown` (`self.BPC_RaffleHandling`)))))

(fn `UpdateCurrentPlayer`
  (bind _viewercube (`/Game/UI/ViewerExclusive/WB_ViewerHUD.ViewerCube` (`/Game/UI/ViewerExclusive/WB_ViewerPerspective.WB_ViewerHUD` (`self.ViewerHUD`))))
  ;[1 1 1] Find currently selected user
  (for (_array_element _array_index) (`PanelWidget.GetAllChildren` (`/Game/UI/GeneralUI/WB_PlayerIconDisplay.PictureLine` (`/Game/UI/ViewerExclusive/WB_ViewerPerspective.PlayerIconsBox` (`self.ViewerHUD`))))
    (bind _aswb_icon (cast `/Game/UI/GeneralUI/WB_Icon` _array_element))
    (if (!= _array_index (`self.SelectedPlayer`))
      ;[1 1 1] Change Selected User Background To Unselected
      (`/Game/UI/GeneralUI/WB_Icon.UpdateOutline` _aswb_icon (`KismetMathLibrary.Conv_LinearColorToColor` (`KismetMathLibrary.LinearColor_White`)))
      (else
        ;[1 1 1] Change User Selected Background To Selected
        (`/Game/UI/GeneralUI/WB_Icon.UpdateOutline` _aswb_icon (`KismetMathLibrary.Conv_LinearColorToColor` (`KismetMathLibrary.LinearColor_Blue`)))
        (if (> (break `LinearColor` (break `SlateColor` (`.TintColor` (break `SlateBrush` (`Border.Background` (`/Game/UI/GeneralUI/WB_Icon.PlayingBorder` _aswb_icon)))))) 0.0)
          (`Widget.SetIsEnabled` _viewercube false)
          (else
            (`Widget.SetIsEnabled` _viewercube true)))))))

(fn `UpdateLB`
  (locals (`Ordered list` :type "Array of Integer") (Players :type Integer) (FirstPass :type Boolean :default true))
  (for _array_element (`self.ExamplePlayers`)
    (if (`.Participating_16_2FB093A24519A01D14EE788F67F6B3C1` (break `/Game/GameData/STRUCT_Viewer` _array_element))
      (set `local.Players` (+ (`local.Players`) 1))
      (if (`local.FirstPass`)
        ;[1 1 1] Initialise list
        (`KismetArrayLibrary.Array_Add` (`local.Ordered list`) (`.ID_8_BA49C3F345E774A3080E77B342852339` (break `/Game/GameData/STRUCT_Viewer` _array_element)))
        (set `local.FirstPass` false)
        (else
          ;[1 1 1] Check if player has a score high enough for the leaderboard
          (for (_array_element_2 _array_index) (`local.Ordered list`)
            (bind (_output_username _output_profilepicture _output_id _output_score) (break `/Game/GameData/STRUCT_Viewer` (`|GetArrayItem` (`self.ExamplePlayers`) _array_element_2)))
            (if (>= _output_score (`.Score_11_B902EE6E4C2986D6DB2CF4A63004A1DE` (break `/Game/GameData/STRUCT_Viewer` _array_element)))
              (`KismetArrayLibrary.Array_Insert` (`local.Ordered list`) (`.ID_8_BA49C3F345E774A3080E77B342852339` (break `/Game/GameData/STRUCT_Viewer` _array_element)) _array_index)
              (break)))
          ;[1 1 1] Add to the end of the list if not greater than any value
          (if (!= (`KismetArrayLibrary.Array_Length` (`local.Ordered list`)) (+ (`.ID_8_BA49C3F345E774A3080E77B342852339` (break `/Game/GameData/STRUCT_Viewer` _array_element)) 1))
            (`KismetArrayLibrary.Array_Add` (`local.Ordered list`) (`.ID_8_BA49C3F345E774A3080E77B342852339` (break `/Game/GameData/STRUCT_Viewer` _array_element))))))))
  ;[1 1 1] Update visual top 4
  (for _index (range 3 1)
    (`KismetArrayLibrary.Array_Set` (`self.TopPlayers`) _index (`|GetArrayItem` (`local.Ordered list`) _index)))
  (set `/Game/BPC_Elimination.PlayersOrdered` (`local.Ordered list`) (`self.BPC_Elimination`)))

(fn `UpdateLeaderboard`
  (params (ID :type "Integer (by ref)") (Score :type Integer))
  (locals (Updated :type Boolean))
  ;[1 1 1] Loop Through whole leaderboard
  (for (_array_element _array_index) (`self.TopPlayers`)
    (bind (_output_username _output_profilepicture _output_id _output_score) (break `/Game/GameData/STRUCT_Viewer` (`|GetArrayItem` (`self.ExamplePlayers`) _array_element)))
    (if (!= ID _output_id)
      (if (> Score _output_score)
        (`self.InputPlayerLB` _array_index)
        (`KismetArrayLibrary.Array_Set` (`self.TopPlayers`) _array_index ID)
        (break))
      (else
        (break)))))

(fn `UserConstructionScript`)