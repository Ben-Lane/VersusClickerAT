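; Game mode component that runs timed elimination rounds between the streamer and viewers until one winner remains.
; While playing, Tick counts up to EliminationTime, refreshes the leaderboard through GM_MainGameMode, then eliminates and restarts after a short delay.
; EliminatePlayer compares the streamer's score with the first PlayersOrdered viewer, treated as lowest, and briefly flags the eliminated name for display.
; EndGame stores the winner's name and calls the game mode's GameEnd after a delay.
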(event `self.ReceiveTick`
  (params (DeltaSeconds :type "Float (single-precision)"))
  (if (`self.PlayingStarted`)
    (bind _output_get (set `self.ElapsedTime` (+ (`self.ElapsedTime`) DeltaSeconds)))
    (if (>= _output_get (`self.EliminationTime`))
      (bind _asgm_main_game_mode (cast `/Game/GM_MainGameMode` (`self.GetOwner`)))
      (`/Game/GM_MainGameMode.UpdateLB` _asgm_main_game_mode)
      ;[1 1 1] Eliminate player
      (`self.EliminatePlayer`)
      (set `self.ElapsedTime` 0.0)
      (set `self.PlayingStarted` false)
      (`self.StartEliminationProcess`))))

(event `StartEliminationProcess`
  ;[1 1 1] Starts Elimination Cycle
  (`KismetSystemLibrary.Delay` 1.0)
  (set `self.PlayingStarted` true)
  (if (<= (`KismetArrayLibrary.Array_Length` (`self.PlayersOrdered`)) 0)
    (`self.EndGame` "Streamer")))

(event `ShowEliminatedPlayerText`
  (set `self.EliminationBeingShown` true)
  (`KismetSystemLibrary.Delay` 2.0)
  (set `self.EliminationBeingShown` false))

(event `EndGame`
  (params (Winner :type Text))
  (set `self.WinnerName` Winner)
  ;[1 1 1] Triggers Game Ending State
  (set `self.PlayingStarted` false)
  (`KismetSystemLibrary.Delay` 2.0)
  (bind _asgm_main_game_mode (cast `/Game/GM_MainGameMode` (`self.GetOwner`)))
  (`/Game/GM_MainGameMode.GameEnd` _asgm_main_game_mode))

(fn `EliminatePlayer`
  (bind _playersordered (`self.PlayersOrdered`))
  (bind _playersordered_2 (`self.PlayersOrdered`))
  (bind _asgm_main_game_mode (cast `/Game/GM_MainGameMode` (`self.GetOwner`)))
  (if (`/Game/GM_MainGameMode.StreamerParticipating` _asgm_main_game_mode)
    ;[1 1 1] Find Player with lowest score
    (bind _asbp_streamer_data_gi (cast `/Game/GameData/BP_StreamerDataGI` (`GameplayStatics.GetGameInstance`)))
    (bind (_output_username _output_profilepicture _output_id _output_score) (break `/Game/GameData/STRUCT_Viewer` (`|GetArrayItem` (`/Game/GM_MainGameMode.ExamplePlayers` _asgm_main_game_mode) (`|GetArrayItem` (`self.PlayersOrdered`)))))
    (if (< (`/Game/GameData/BP_StreamerDataGI.StreamerScore` _asbp_streamer_data_gi) _output_score)
      (set `/Game/GM_MainGameMode.StreamerParticipating` false _asgm_main_game_mode)
      (set `self.EliminationName` "Streamer")
      (`self.ShowEliminatedPlayerText`)
      (if (== (`KismetArrayLibrary.Array_Length` (`self.PlayersOrdered`)) 1)
        ;[0.007438 1 0] Last remaining viewer wins
        (`KismetSystemLibrary.PrintString` "Final Viewer Wins")
        (bind _asgm_main_game_mode_2 (cast `/Game/GM_MainGameMode` (`GameplayStatics.GetGameMode`)))
        (bind _output_username_2 (break `/Game/GameData/STRUCT_Viewer` (`|GetArrayItem` (`/Game/GM_MainGameMode.ExamplePlayers` _asgm_main_game_mode_2) (`|GetArrayItem` _playersordered_2 (`KismetArrayLibrary.Array_LastIndex` _playersordered_2)))))
        (`self.EndGame` (`KismetTextLibrary.Conv_StringToText` _output_username_2))
        (else
          (`KismetSystemLibrary.PrintString` "Case 1")))
      (else
        (bind _exampleplayers (`/Game/GM_MainGameMode.ExamplePlayers` _asgm_main_game_mode))
        (bind (_output_username_3 _output_profilepicture_2 _output_id_2 _output_score_2 _output_scoreaddition _output_participating _output_scorecalculator) (break `/Game/GameData/STRUCT_Viewer` (`|GetArrayItem` _exampleplayers (`|GetArrayItem` (`self.PlayersOrdered`)))))
        (`KismetArrayLibrary.Array_Set` _exampleplayers _output_id_2 (make `/Game/GameData/STRUCT_Viewer` _output_username_3 _output_profilepicture_2 _output_id_2 _output_score_2 _output_scoreaddition false _output_scorecalculator) :!label _label)
        (set `self.EliminationName` (`KismetTextLibrary.Conv_StringToText` _output_username_3))
        (`self.ShowEliminatedPlayerText`)
        (if (== (`KismetArrayLibrary.Array_Length` (`self.PlayersOrdered`)) 1)
          ;[0.0402 1 0] Streamer wins
          (`KismetSystemLibrary.PrintString` "Streamer Wins (last alive)")
          (`self.EndGame` "Streamer")
          (elif (== (`KismetArrayLibrary.Array_Length` (`self.PlayersOrdered`)) 2)
            (if (`/Game/GM_MainGameMode.StreamerParticipating` _asgm_main_game_mode)
              (`KismetSystemLibrary.PrintString` "Case 2")
              (else
                ;[0.007438 1 0] Last remaining viewer wins
                (`KismetSystemLibrary.PrintString` "Final Viewer Wins")
                (bind _asgm_main_game_mode_3 (cast `/Game/GM_MainGameMode` (`GameplayStatics.GetGameMode`)))
                (bind _output_username_4 (break `/Game/GameData/STRUCT_Viewer` (`|GetArrayItem` (`/Game/GM_MainGameMode.ExamplePlayers` _asgm_main_game_mode_3) (`|GetArrayItem` _playersordered (`KismetArrayLibrary.Array_LastIndex` _playersordered)))))
                (`self.EndGame` (`KismetTextLibrary.Conv_StringToText` _output_username_4))))
            (else
              (`KismetSystemLibrary.PrintString` "Case 3"))))))
    (else
      (goto _label))))